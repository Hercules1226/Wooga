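; BP_PlaneMask is an Easy Dissolve actor whose moving plane defines a mask for materials.
; It writes the plane's world location and up vector to the MPC_PlaneMask parameter collection, both on construction and every tick.
; From BeginPlay, the Movement timeline drives the plane's world X at a hardcoded Y and Z.
; A second timeline, played from Tick, animates the plane material's Opacity.
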(event `self.ReceiveTick`
  (params (DeltaSeconds :type "Float (single-precision)"))
  (bind _plane (`self.Plane`))
  (`KismetMaterialLibrary.SetVectorParameterValue` "/Game/EasyDissolve/Materials/CollectionParameters/MPC_PlaneMask.MPC_PlaneMask" "Location_1" (`KismetMathLibrary.Conv_VectorToLinearColor` (`SceneComponent.K2_GetComponentLocation` _plane)))
  (`KismetMaterialLibrary.SetVectorParameterValue` "/Game/EasyDissolve/Materials/CollectionParameters/MPC_PlaneMask.MPC_PlaneMask" "Rotation_1" (`KismetMathLibrary.Conv_VectorToLinearColor` (`SceneComponent.GetUpVector` _plane)))
  (bind (_direction _newtrack_0) (`Timeline|Timeline_0`)
    (:`Update`
      (`MeshComponent.SetScalarParameterValueOnMaterials` (`self.Plane`) "Opacity" _newtrack_0))))

(event `self.ReceiveBeginPlay`
  (bind (_direction _newtrack_0) (`Timeline|Movement`)
    (:`Update`
      (`SceneComponent.K2_SetWorldLocation` (`self.Plane`) (`KismetMathLibrary.MakeVector` _newtrack_0 2000.0 220.0) false false))))

(fn `UserConstructionScript`
  (bind _plane (`self.Plane`))
  (`KismetMaterialLibrary.SetVectorParameterValue` "/Game/EasyDissolve/Materials/CollectionParameters/MPC_PlaneMask.MPC_PlaneMask" "Location_1" (`KismetMathLibrary.Conv_VectorToLinearColor` (`SceneComponent.K2_GetComponentLocation` _plane)))
  (`KismetMaterialLibrary.SetVectorParameterValue` "/Game/EasyDissolve/Materials/CollectionParameters/MPC_PlaneMask.MPC_PlaneMask" "Rotation_1" (`KismetMathLibrary.Conv_VectorToLinearColor` (`SceneComponent.GetUpVector` _plane))))