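; Butterfly actor that alternates between idling at spline points and flying to the next one, wrapping back to the first.
; A randomly chosen idle timeline leads into a flight timeline that blends location axes separately and turns toward the travel direction.
; Timelines drive wing animation through dynamic material parameters, with colour set at construction.
; TriggerNext interrupts idling to start the next flight.
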(event `TriggerNext`
  (bind _currentsplinepoint (`self.CurrentSplinePoint`))
  (bind _butterflymaterial (`self.ButterflyMaterial`))
  (bind _starttransform (`self.StartTransform`))
  (bind _targettransform (`self.TargetTransform`))
  (bind _targettransform_location (`KismetMathLibrary.BreakTransform` (`self.TargetTransform`)))
  (bind _starttransform_location (`KismetMathLibrary.BreakTransform` (`self.StartTransform`)))
  ;[1 1 1] Interrupt Idle and Trigger Next Flight
  (`|ExecutionSequence`
    (:`then_0`
      ;[1 1 1] IdleAnimations
      (bind (_direction _time) (`Timeline|Idle_03` :!via `Stop` :!label _label)
        (:`Update`
          (`MaterialInstanceDynamic.SetScalarParameterValue` (`self.ButterflyMaterial`) "Manual_Time" _time))
        (:`Finished`
          ;[1 1 1] Get Next Point Location
          (bind _result (`/Engine/EditorBlueprintResources/StandardMacros.IncrementInt` _currentsplinepoint :!label _label_2)
            (:`  `
              (if (>= _result (`SplineComponent.GetNumberOfSplinePoints` (`self.Spline`)))
                (set `self.CurrentSplinePoint` 0))
              (set `self.TargetTransform` (`SplineComponent.GetTransformAtSplinePoint` (`self.Spline`) _currentsplinepoint "Local" false))
              ;[1 1 1] Flying
              (bind (_direction_2 _lerp_xy _lerp_z _lerp_rot _time_2 _flightrot _wing_offset) (`Timeline|Flying_01` :!via `PlayFromStart`)
                (:`Update`
                  (`SceneComponent.K2_SetRelativeTransform` (`self.Butterfly`) (`KismetMathLibrary.MakeTransform` (`KismetMathLibrary.MakeVector` (`KismetMathLibrary.Lerp` (.x (.location _starttransform)) (.x (.location _targettransform)) _lerp_xy) (`KismetMathLibrary.Lerp` (.y (.location _starttransform)) (.y (.location _targettransform)) _lerp_xy) (`KismetMathLibrary.Lerp` (.z (.location _starttransform)) (.z (.location _targettransform)) _lerp_z)) (`KismetMathLibrary.RLerp` (`KismetMathLibrary.RLerp` (.rotation _starttransform) (.rotation _targettransform) _lerp_rot true) (`KismetMathLibrary.MakeRotFromX` (- _targettransform_location _starttransform_location)) _flightrot true) (`KismetMathLibrary.Conv_DoubleToVector` (`self.Scale`))) false false)
                  (`MaterialInstanceDynamic.SetScalarParameterValue` _butterflymaterial "Manual_Time" _time_2)
                  (`MaterialInstanceDynamic.SetScalarParameterValue` _butterflymaterial "Wing_Offset" _wing_offset))
                (:`Finished`
                  ;[1 1 1] Loop
                  (set `self.StartTransform` (`self.TargetTransform`))
                  (`self.StartIdle`))))))))
    (:`then_1`
      (bind (_direction_3 _time_3) (`Timeline|Idle_02` :!via `Stop` :!label _label_3)
        (:`Update`
          (`MaterialInstanceDynamic.SetScalarParameterValue` (`self.ButterflyMaterial`) "Manual_Time" _time_3))
        (:`Finished`
          (goto _label_2))))
    (:`then_2`
      (goto _label :!via `Stop`))
    (:`then_3`
      (goto _label_2))))

(event `self.ReceiveBeginPlay`
  ;[1 1 1] Loop Start - Select Random Idle Animations
  (`KismetSystemLibrary.Delay` (`KismetMathLibrary.RandomFloat`))
  (switch `int` (`KismetMathLibrary.RandomIntegerInRange` 0 2) :!label _label_4
    (:`0`
      ;[1 1 1] IdleAnimations
      (bind (_direction _time) (`Timeline|Idle_01` :!via `PlayFromStart`)
        (:`Update`
          (`MaterialInstanceDynamic.SetScalarParameterValue` (`self.ButterflyMaterial`) "Manual_Time" _time))
        (:`Finished`
          (goto _label_2))))
    (:`1`
      (goto _label_3 :!via `PlayFromStart`))
    (:`2`
      (goto _label :!via `PlayFromStart`))))

(event `StartIdle`
  ;[1 1 1] Loop Start - Select Random Idle Animations
  (goto _label_4))

(fn `UserConstructionScript`
  (bind _butterfly (`self.Butterfly`))
  (bind _butterflymaterial (`self.ButterflyMaterial`))
  (bind _spline (`self.Spline`))
  (`|ExecutionSequence`
    (:`then_0`
      ;[1 1 1] Set Up Material
      (bind _returnvalue (`PrimitiveComponent.CreateDynamicMaterialInstance` _butterfly 0 (`PrimitiveComponent.GetMaterial` _butterfly 0) "None"))
      (set `self.ButterflyMaterial` _returnvalue)
      (if (`self.RandomiseColour`)
        (`MaterialInstanceDynamic.SetScalarParameterValue` _butterflymaterial "Randomise_Colours" 0.0)
        (`MaterialInstanceDynamic.SetScalarParameterValue` _butterflymaterial "Colour_Selector" (`KismetMathLibrary.RandomFloat`))
        (else
          (`MaterialInstanceDynamic.SetScalarParameterValue` _butterflymaterial "Randomise_Colours" 0.0)
          (`MaterialInstanceDynamic.SetScalarParameterValue` _butterflymaterial "Colour_Selector" (`self.Colour`)))))
    (:`then_1`
      ;[1 1 1] Set Initial Position
      (set `self.NumberSplinePoints` (`SplineComponent.GetNumberOfSplinePoints` _spline))
      (bind _output_get (set `self.StartTransform` (`SplineComponent.GetTransformAtSplinePoint` _spline 0 "Local" false)))
      (`SceneComponent.K2_SetRelativeTransform` (`self.Butterfly`) (`KismetMathLibrary.MakeTransform` (.location _output_get) (.rotation _output_get) (`KismetMathLibrary.Conv_DoubleToVector` (`self.Scale`))) false false))))