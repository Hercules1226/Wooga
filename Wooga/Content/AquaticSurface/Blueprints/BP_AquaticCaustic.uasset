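; Aquatic caustics decal actor that plays an animated sequence of textures, projected along the sun direction.
; Construction creates a dynamic decal material and derives its DecalSize parameter from a Plane offset.
; Tick interval follows AnimationSpeed, so each tick advances one frame and refreshes sun direction, aligned to an optional LightSource, plus UV axes built from cross products.
; SetInteraction feeds a supplied texture into the material's Heightfield parameter.
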(event `self.ReceiveBeginPlay`
  ;[1 1 1] Update interval optimization
  (`self.SetActorTickInterval` (/ 1.0 (`KismetMathLibrary.FMax` (`self.AnimationSpeed`) 0.01))))

(event `self.ReceiveTick`
  (params (DeltaSeconds :type "Float (single-precision)"))
  ;[1 1 1] Next frame
  (set `self.AnimationFrame` (mod (+ (`self.AnimationFrame`) 1) (`KismetArrayLibrary.Array_Length` (`self.AnimationFrames`))))
  (`self.SetParameters`))

(fn `SetInteraction`
  (params (Texture :type "Texture Object Reference"))
  (`MaterialInstanceDynamic.SetTextureParameterValue` (`self.MaterialInstance`) "Heightfield" Texture))

(fn `SetParameters`
  (bind _lightsource (`self.LightSource`))
  (bind _returnvalue (`SceneComponent.GetForwardVector` (`self.SunDirection`)))
  (bind (_x _y) (`KismetMathLibrary.BreakVector2D` (`self.UVMove`)))
  (bind (_x_2 _y_2) (`KismetMathLibrary.BreakVector2D` (`self.UVScale`)))
  (bind _returnvalue_2 (`KismetMathLibrary.Normal` (`KismetMathLibrary.Cross_VectorVector` _returnvalue (0.0 1.0 0.0))))
  (`/Engine/EditorBlueprintResources/StandardMacros.IsValid` _lightsource
    (:`Is Valid`
      (`SceneComponent.K2_SetWorldRotation` (`self.SunDirection`) (`SceneComponent.K2_GetComponentRotation` (`Light.LightComponent` _lightsource)) false false))
    (:`Is Not Valid`
      _))
  (`MaterialInstanceDynamic.SetTextureParameterValue` (`self.MaterialInstance`) "DecalTexture" (`|GetArrayItem` (`self.AnimationFrames`) (`self.AnimationFrame`)))
  (`MaterialInstanceDynamic.SetVectorParameterValue` (`self.MaterialInstance`) "SunDirection" (`KismetMathLibrary.Conv_VectorToLinearColor` _returnvalue))
  (`MaterialInstanceDynamic.SetVectorParameterValue` (`self.MaterialInstance`) "UVAxisX" (make `LinearColor` (.x (* _returnvalue_2 _x_2)) (.y (* _returnvalue_2 _x_2)) (.z (* _returnvalue_2 _x_2)) _x))
  (`MaterialInstanceDynamic.SetVectorParameterValue` (`self.MaterialInstance`) "UVAxisY" (make `LinearColor` (.x (* (`KismetMathLibrary.Normal` (`KismetMathLibrary.Cross_VectorVector` _returnvalue_2 (0.0 0.0 1.0))) _y_2)) (.y (* (`KismetMathLibrary.Normal` (`KismetMathLibrary.Cross_VectorVector` _returnvalue_2 (0.0 0.0 1.0))) _y_2)) (.z (* (`KismetMathLibrary.Normal` (`KismetMathLibrary.Cross_VectorVector` _returnvalue_2 (0.0 0.0 1.0))) _y_2)) _y)))

(fn `UserConstructionScript`
  (bind _lightsource (`self.LightSource`))
  (`SceneComponent.K2_SetRelativeLocation` (`self.Plane`) (`KismetMathLibrary.MakeVector` (.x (`DecalComponent.DecalSize` (`self.Decal`)))) false false)
  (bind _returnvalue (`KismetMaterialLibrary.CreateDynamicMaterialInstance` (`self.Decal`) (`self.DynamicMaterial`)))
  (bind _output_get (set `self.MaterialInstance` _returnvalue))
  (`DecalComponent.SetDecalMaterial` (`self.Decal`) _output_get)
  (`self.SetParameters`)
  (`MaterialInstanceDynamic.SetScalarParameterValue` (`self.MaterialInstance`) "DecalSize" (.z (- (`SceneComponent.K2_GetComponentLocation` (`self.Plane`)) (`SceneComponent.K2_GetComponentLocation` (`self.Decal`)))))
  (`/Engine/EditorBlueprintResources/StandardMacros.IsValid` _lightsource
    (:`Is Valid`
      (`SceneComponent.K2_SetWorldRotation` (`self.SunDirection`) (`SceneComponent.K2_GetComponentRotation` (`Light.LightComponent` _lightsource)) false false))))