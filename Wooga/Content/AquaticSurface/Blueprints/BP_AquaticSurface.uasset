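; BP_AquaticSurface is a placeable water body with over/under surface materials, an underwater post-process volume, underwater audio and cuttable holes.
; Construction builds dynamic materials, sizes the volumes and sets up box-projected cubemap and optional planar reflections.
; Overlaps assign the volume to buoyancy components and register actors both in view and on the surface with AquaticSimulation.
; A timer updates shared fog and height parameters from the highest-priority surface near the camera, flipping the planar reflection underwater.
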(event `CaptureEvent`
  (bind _capturecube (`self.CaptureCube`))
  ;[1 1 1] Post begin initialize components
  (`self.UpdateVolume`)
  (if (>= (`self.ReflectionCaptureDelay`) 0.0) :!label _label
    (`KismetSystemLibrary.Delay` (`self.ReflectionCaptureDelay`))
    (`/Engine/EditorBlueprintResources/StandardMacros.IsValid` _capturecube
      (:`Is Valid`
        (`SceneCaptureComponentCube.CaptureScene` _capturecube)))))

(event `self.PostProcessShape.OnComponentBeginOverlap`
  (params (OverlappedComponent :type "PrimitiveComponent Object Reference") (OtherActor :type "Actor Object Reference") (OtherComp :type "PrimitiveComponent Object Reference") (OtherBodyIndex :type Integer) (bFromSweep :type Boolean) (SweepResult :type "HitResult Structure (by ref)"))
  ;[1 1 1] Overlap events
  (`self.OnBeginOverlapBuoyancy` OtherActor))

(event `self.ReceiveBeginPlay`
  (bind _cameraupdatefrequency (`self.CameraUpdateFrequency`))
  ;[1 1 1] Post begin initialize components
  (`self.UpdateHoles`)
  (`|ExecutionSequence`
    (:`then_0`
      (`|ExecutionSequence`
        (:`then_0`
          (goto _label))
        (:`then_1`
          (`self.UpdateVolume`))))
    (:`then_1`
      ;[1 1 1] Overlap actors
      (`KismetSystemLibrary.Delay` 0.0)
      (for _array_element (`PrimitiveComponent.GetOverlappingActors` (`self.PostProcessShape`) null)
        (`self.OnBeginOverlapBuoyancy` _array_element)))
    (:`then_2`
      (`KismetSystemLibrary.Delay` 0.0)
      (for _array_element_2 (`PrimitiveComponent.GetOverlappingActors` (`self.InteractionView`) null)
        (`self.OnBeginOverlapInteraction` _array_element_2 (`self.InteractionsInView`))))
    (:`then_3`
      (`KismetSystemLibrary.Delay` 0.0)
      (for _array_element_3 (`PrimitiveComponent.GetOverlappingActors` (`self.PlaneOverWater`) null)
        (`self.OnBeginOverlapInteraction` _array_element_3 (`self.InteractionsOnSurface`))))
    (:`then_4`
      ;[1 1 1] Camera overlaping update
      (if (> _cameraupdatefrequency 0.0)
        (`KismetSystemLibrary.K2_SetTimerDelegate` (delegate `UpdateCameraEvent`) _cameraupdatefrequency true)))))

(event `self.PostProcessShape.OnComponentEndOverlap`
  (params (OverlappedComponent :type "PrimitiveComponent Object Reference") (OtherActor :type "Actor Object Reference") (OtherComp :type "PrimitiveComponent Object Reference") (OtherBodyIndex :type Integer))
  ;[1 1 1] Overlap events
  (`self.OnEndOverlapBuoyancy` OtherActor))

(event `self.InteractionView.OnComponentBeginOverlap`
  (params (OverlappedComponent :type "PrimitiveComponent Object Reference") (OtherActor :type "Actor Object Reference") (OtherComp :type "PrimitiveComponent Object Reference") (OtherBodyIndex :type Integer) (bFromSweep :type Boolean) (SweepResult :type "HitResult Structure (by ref)"))
  ;[1 1 1] Interaction overlap
  (`self.OnBeginOverlapInteraction` OtherActor (`self.InteractionsInView`)))

(event `UpdateCameraEvent`
  ;[1 1 1] Camera overlaping update
  (`self.OverlapCamera`))

(event `self.InteractionView.OnComponentEndOverlap`
  (params (OverlappedComponent :type "PrimitiveComponent Object Reference") (OtherActor :type "Actor Object Reference") (OtherComp :type "PrimitiveComponent Object Reference") (OtherBodyIndex :type Integer))
  ;[1 1 1] Interaction overlap
  (`self.OnEndOverlapInteraction` OtherActor (`self.InteractionsInView`)))

(event `self.PlaneOverWater.OnComponentBeginOverlap`
  (params (OverlappedComponent :type "PrimitiveComponent Object Reference") (OtherActor :type "Actor Object Reference") (OtherComp :type "PrimitiveComponent Object Reference") (OtherBodyIndex :type Integer) (bFromSweep :type Boolean) (SweepResult :type "HitResult Structure (by ref)"))
  ;[1 1 1] Interaction overlap
  (`self.OnBeginOverlapInteraction` OtherActor (`self.InteractionsOnSurface`)))

(event `/Game/AquaticSurface/Blueprints/BPI_AqiatocWorld.OnWorldOriginChanged`
  (params (`Old Origin` :type "IntVector Structure") (`New Origin` :type "IntVector Structure"))
  ;[1 1 1] World origin changed
  (`self.UpdateCubemapParameters`))

(event `self.PlaneOverWater.OnComponentEndOverlap`
  (params (OverlappedComponent :type "PrimitiveComponent Object Reference") (OtherActor :type "Actor Object Reference") (OtherComp :type "PrimitiveComponent Object Reference") (OtherBodyIndex :type Integer))
  ;[1 1 1] Interaction overlap
  (`self.OnEndOverlapInteraction` OtherActor (`self.InteractionsOnSurface`)))

(fn `BoxReflection`
  (params (BoxShape :type "BoxComponent Object Reference") (UseMaterial :type "MaterialInstanceDynamic Object Reference") (BoxExtent :type "Vector Structure") (BoxLocation :type "Vector Structure") (Over :type Boolean))
  (bind _usematerial (`local.UseMaterial`))
  (bind _staticreflectioncubemap (`self.StaticReflectionCubemap`))
  (bind _returnvalue (* (`BoxComponent.GetScaledBoxExtent` (`local.BoxShape`)) (1.0 1.0 2.0)))
  (bind _returnvalue_2 (+ (* (`local.BoxLocation`) (`SceneComponent.RelativeScale3D` (`self.Root`))) (`self.K2_GetActorLocation`)))
  ;[1 1 1] Update preview
  (`SceneComponent.K2_SetRelativeLocation` (`local.BoxShape`) (- (`local.BoxLocation`) (`KismetMathLibrary.MakeVector` 0.0 0.0 (* (.z BoxExtent) (select `bool` Over :`false` 0.5 :`true` -0.5 :!type "Float (single-precision)")))) false true)
  (`BoxComponent.SetBoxExtent` (`local.BoxShape`) (* (`local.BoxExtent`) (1.0 1.0 0.5)) true)
  (`SceneComponent.SetRelativeScale3D` (`local.BoxShape`) (1.0 1.0 1.0))
  ;[1 1 1] Update material
  (`MaterialInstanceDynamic.SetVectorParameterValue` _usematerial "BoxProjectionMin" (`KismetMathLibrary.Conv_VectorToLinearColor` (- _returnvalue_2 _returnvalue)))
  (`MaterialInstanceDynamic.SetVectorParameterValue` _usematerial "BoxProjectionMax" (`KismetMathLibrary.Conv_VectorToLinearColor` (+ _returnvalue_2 _returnvalue)))
  (`MaterialInstanceDynamic.SetVectorParameterValue` _usematerial "BoxProjectionPos" (`KismetMathLibrary.Conv_VectorToLinearColor` (+ (`self.ReflectionLocation`) (`SceneComponent.K2_GetComponentLocation` (`self.Root`)))))
  (`/Engine/EditorBlueprintResources/StandardMacros.IsValid` _staticreflectioncubemap
    (:`Is Valid`
      (`MaterialInstanceDynamic.SetTextureParameterValue` _usematerial "Cubemap" _staticreflectioncubemap))))

(fn `GetHeight`
  (returns (Height :type "Float (double-precision)"))
  (bind (_returnvalue_x _returnvalue_y _returnvalue_z) (`KismetMathLibrary.BreakVector` (`SceneComponent.K2_GetComponentLocation` (`self.Root`))))
  (return _returnvalue_z))

(fn `InitMaterials`
  (`|ExecutionSequence`
    (:`then_0`
      ;[1 1 1] Port process material
      (`/Engine/EditorBlueprintResources/StandardMacros.IsValid` (`self.ScreenMaterial`)
        (:`Is Valid`
          (bind _returnvalue (`PrimitiveComponent.CreateDynamicMaterialInstance` (`self.PlaneTopDown`) 0 (`self.ScreenMaterial`)))
          (bind _output_get (set `self.ScreenMaterialIntance` _returnvalue))
          (`PostProcessComponent.AddOrUpdateBlendable` (`self.PostProcess`) _output_get 1.0))))
    (:`then_1`
      ;[1 1 1] Topdown material
      (`/Engine/EditorBlueprintResources/StandardMacros.IsValid` (`self.TopDownMaterial`)
        (:`Is Valid`
          (bind _returnvalue_2 (`PrimitiveComponent.CreateDynamicMaterialInstance` (`self.PlaneTopDown`) 0 (`self.TopDownMaterial`)))
          (set `self.TopDownMaterialInstance` _returnvalue_2))
        (:`Is Not Valid`
          (`ActorComponent.K2_DestroyComponent` (`self.PlaneTopDown`)))))
    (:`then_2`
      ;[1 1 1] Surface material
      (bind _returnvalue_3 (`PrimitiveComponent.CreateDynamicMaterialInstance` (`self.PlaneOverWater`) 0 (`self.OverWaterMaterial`)))
      (set `self.OverWaterMaterialInstance` _returnvalue_3)
      (bind _returnvalue_4 (`PrimitiveComponent.CreateDynamicMaterialInstance` (`self.PlaneUnderWater`) 0 (`self.UnderWaterMaterial`)))
      (set `self.UnderWaterMaterialInstance` _returnvalue_4)
      (bind _returnvalue_5 (`PrimitiveComponent.CreateDynamicMaterialInstance` (`self.PostProcessMesh`) 0 (`self.VolumeMaterial`)))
      (set `self.VolumeMaterialInstance` _returnvalue_5)
      (return))))

(fn `InitReflectionPlane`
  (if (`self.UseReflectionPlane`)
    (set `SceneCaptureComponent.HiddenActors` (`self.HiddenInReflection`) (`self.PlanarReflection`))
    (else
      (`/Engine/EditorBlueprintResources/StandardMacros.IsValid` (`self.PlanarReflection`)
        (:`Is Valid`
          (`ActorComponent.K2_DestroyComponent` (`self.PlanarReflection`)))))))

(fn `OnBeginOverlapBuoyancy`
  (params (OtherActor :type "Actor Object Reference"))
  (bind _returnvalue (`self.GetComponentByClass` OtherActor "/Game/AquaticSurface/Blueprints/BP_AquaticBuoyancy.BP_AquaticBuoyancy_C"))
  (if (`KismetSystemLibrary.IsValid` _returnvalue)
    (`/Game/AquaticSurface/Blueprints/BP_AquaticBuoyancy.SetAquaticVolume` _returnvalue self)))

(fn `OnBeginOverlapInteraction`
  (params (OtherActor :type "Actor Object Reference") (List :type "Array of Actor Object Reference (by ref)"))
  (if (`KismetSystemLibrary.IsValid` (`self.AquaticSimulation`))
    (`KismetArrayLibrary.Array_Add` List OtherActor)
    (if (and (>= (`KismetArrayLibrary.Array_Find` (`self.InteractionsInView`) OtherActor) 0) (>= (`KismetArrayLibrary.Array_Find` (`self.InteractionsOnSurface`) OtherActor) 0))
      (`/Game/AquaticSurface/Blueprints/BP_AquaticSimulation.AddInteractionActor` (`self.AquaticSimulation`) self (`local.OtherActor`)))))

(fn `OnEndOverlapBuoyancy`
  (params (OtherAtor :type "Actor Object Reference"))
  (bind _returnvalue (`self.GetComponentByClass` OtherAtor "/Game/AquaticSurface/Blueprints/BP_AquaticBuoyancy.BP_AquaticBuoyancy_C"))
  (if (`KismetSystemLibrary.IsValid` _returnvalue)
    (if (== (`/Game/AquaticSurface/Blueprints/BP_AquaticBuoyancy.InWater` _returnvalue) self)
      (`/Game/AquaticSurface/Blueprints/BP_AquaticBuoyancy.SetAquaticVolume` _returnvalue null))))

(fn `OnEndOverlapInteraction`
  (params (OtherAtor :type "Actor Object Reference") (List :type "Array of Actor Object Reference (by ref)"))
  (if (`KismetSystemLibrary.IsValid` (`self.AquaticSimulation`))
    (if (and (>= (`KismetArrayLibrary.Array_Find` (`self.InteractionsInView`) (`local.OtherAtor`)) 0) (>= (`KismetArrayLibrary.Array_Find` (`self.InteractionsOnSurface`) (`local.OtherAtor`)) 0))
      (`/Game/AquaticSurface/Blueprints/BP_AquaticSimulation.RemoveInteractionActor` (`self.AquaticSimulation`) (`local.OtherAtor`)))
    (`KismetArrayLibrary.Array_RemoveItem` List (`local.OtherAtor`))))

(fn `OverlapCamera`
  (locals (PriorityActor :type "/Game/AquaticSurface/Blueprints/BP_AquaticSurface Object Reference") (PriorityValue :type "Float (double-precision)"))
  (bind _returnvalue (`GameplayStatics.GetPlayerCameraManager` 0))
  (bind (_returnvalue_x _returnvalue_y _returnvalue_z) (`KismetMathLibrary.BreakVector` (`PlayerCameraManager.GetCameraLocation` (`GameplayStatics.GetPlayerCameraManager` 0))))
  (bind (_returnvalue_x_2 _returnvalue_y_2 _returnvalue_z_2) (`KismetMathLibrary.BreakVector` (`SceneComponent.K2_GetComponentLocation` (`self.Root`))))
  ;[1 1 1] Find volue closest to the camera and update.
  (`/Engine/EditorBlueprintResources/StandardMacros.IsValid` _returnvalue
    (:`Is Valid`
      (set `local.PriorityActor` null)
      (bind _outactors (`KismetSystemLibrary.BoxOverlapActors` (`PlayerCameraManager.GetCameraLocation` _returnvalue) (50.0 50.0 1500.0) (`|MakeArray` "ObjectTypeQuery2" :!type "EObjectTypeQuery Enum") "BP_AquaticSurface_C"))
      (for _array_element _outactors
        (bind _asbp_aquatic_surface (cast `/Game/AquaticSurface/Blueprints/BP_AquaticSurface` _array_element))
        (bind _priority (`PostProcessComponent.Priority` (`/Game/AquaticSurface/Blueprints/BP_AquaticSurface.PostProcess` _asbp_aquatic_surface)))
        (if (or (== (`local.PriorityActor`) null) (>= _priority (`local.PriorityValue`)))
          (set `local.PriorityActor` _asbp_aquatic_surface)
          (set `local.PriorityValue` _priority)))
      (`/Engine/EditorBlueprintResources/StandardMacros.IsValid` (`local.PriorityActor`)
        (:`Is Valid`
          (`self.UpdateVolume` (`local.PriorityActor`))
          ;;[1 1 1] Inverse reflection plane when camera is under water - hacky way to use single reflection plane :)
          (`/Engine/EditorBlueprintResources/StandardMacros.IsValid` (`self.PlanarReflection`)
            (:`Is Valid`
              (`SceneComponent.K2_SetWorldRotation` (`self.PlanarReflection`) (`KismetMathLibrary.MakeRotator` 0.0 (select `bool` (> _returnvalue_z_2 _returnvalue_z) :`true` 180.0 :!type "Float (single-precision)")) false false))))
        (:`Is Not Valid`
          (`KismetMaterialLibrary.SetScalarParameterValue` "/Game/AquaticSurface/Materials/PC_AquaticSurface.PC_AquaticSurface" "CurrentWaterHeight" -1000.0)
          (`/Engine/EditorBlueprintResources/StandardMacros.IsValid` (`self.PlanarReflection`)
            (:`Is Valid`
              (`SceneComponent.K2_SetWorldRotation` :`self` (`self.PlanarReflection`)))))))))

(fn `PlaySplashEffectByIndex`
  (params (Index :type Integer) (SplashLocation :type "Vector Structure") (SplashScale :type "Float (double-precision)") (SplashVelocity :type "Float (double-precision)"))
  (bind _splasheffects (`self.SplashEffects`))
  (bind (_output_velocitymin _output_velocitymax _output_scalemin _output_scalemax _output_splasheffect _output_splashsound) (break `/Game/AquaticSurface/Blueprints/BS_AquaticSplash` (`|GetArrayItem` _splasheffects)))
  ;[1 1 1] Override this function if you have your method for selecting the splash effect.
  (if (`KismetArrayLibrary.Array_IsValidIndex` _splasheffects Index)
    (if (> SplashVelocity _output_velocitymin)
      (`|ExecutionSequence`
        (:`then_0`
          (if (!= _output_splasheffect null)
            (bind _returnvalue (`GameplayStatics.SpawnEmitterAtLocation` _output_splasheffect (`local.SplashLocation`) (struct) (`KismetMathLibrary.Conv_DoubleToVector` (* (`local.SplashScale`) (`KismetMathLibrary.MapRangeClamped` SplashVelocity _output_velocitymin _output_velocitymax _output_scalemin _output_scalemax)))))
            (`ParticleSystemComponent.SetMaterialParameter` _returnvalue "None" "/Engine/MaterialTemplates/VertexAnimation/AdvancedFlag.AdvancedFlag")))
        (:`then_1`
          (if (!= null _output_splashsound)
            (`GameplayStatics.PlaySoundAtLocation` _output_splashsound (`local.SplashLocation`))
            (return)))))))

(fn `Reconstruct`
  (bind _root (`self.Root`))
  (set `PostProcessComponent.Priority` (`self.PostProcessPriority`) (`self.PostProcess`))
  (`self.InitReflectionPlane`)
  (`SceneComponent.SetVisibility` (`self.PostProcessMesh`) (`self.ShowVolumeMesh`) false)
  (`SceneComponent.SetWorldScale3D` _root (`KismetMathLibrary.MakeVector` (.x (`SceneComponent.K2_GetComponentScale` _root)) (.y (`SceneComponent.K2_GetComponentScale` _root)) 1.0))
  (`self.InitMaterials`)
  (`self.UpdatePostProcessShape`)
  (`self.UpdateReflectionShape`)
  (`self.UpdateCubemapParameters`)
  (`self.UpdateVolume`)
  (`self.UpdateAudioVolume`)
  (`KismetMaterialLibrary.SetScalarParameterValue` "/Game/AquaticSurface/Materials/PC_AquaticSurface.PC_AquaticSurface" "CurrentWaterHeight" -1000.0)
  (`self.CaptureEvent`)
  (`/Engine/EditorBlueprintResources/StandardMacros.IsValid` (`self.AquaticSimulation`)
    (:`Is Valid`
      (if (<= (`KismetArrayLibrary.Array_Find` (`/Game/AquaticSurface/Blueprints/BP_AquaticSimulation.AquaticSurfaces` (`self.AquaticSimulation`)) self) 0)
        _))))

(fn `SetInteraction`
  (params (Value :type "Texture Object Reference"))
  (`MaterialInstanceDynamic.SetTextureParameterValue` (`self.OverWaterMaterialInstance`) "Heightfield" Value)
  (`MaterialInstanceDynamic.SetTextureParameterValue` (`self.UnderWaterMaterialInstance`) "Heightfield" Value))

(fn `UpdateAudioVolume`
  (bind _audiounderwater (`self.AudioUnderwater`))
  (bind _audiounderwater_2 (`self.AudioUnderwater`))
  (bind _outattenuationsettings (`AudioComponent.BP_GetAttenuationSettingsToApply` _audiounderwater))
  (set `AudioComponent.bOverrideAttenuation` true _audiounderwater_2)
  (bind (_battenuate _bspatialize _battenuatewithlpf _benablelistenerfocus _benablefocusinterpolation _benableocclusion _busecomplexcollisionforocclusion _benablereverbsend _bapplynormalizationtostereosounds _benablelogfrequencyscaling _omniradius _stereospread _spatializationalgorithm _spatializationpluginsettings _lpfradiusmin _lpfradiusmax _absorptionmethod _customlowpassairabsorptioncurve _customhighpassairabsorptioncurve _lpffrequencyatmin _lpffrequencyatmax _hpffrequencyatmin _hpffrequencyatmax _focusazimuth _nonfocusazimuth _focusdistancescale _nonfocusdistancescale _focuspriorityscale _nonfocuspriorityscale _focusvolumeattenuation _nonfocusvolumeattenuation _focusattackinterpspeed _focusreleaseinterpspeed _occlusiontracechannel _occlusionlowpassfilterfrequency _occlusionvolumeattenuation _occlusioninterpolationtime _occlusionpluginsettings _reverbsendmethod _reverbpluginsettings _reverbwetlevelmin _reverbwetlevelmax _reverbdistancemin _reverbdistancemax _customreverbsendcurve _manualreverbsendlevel _distancealgorithm _customattenuationcurve _attenuationshape _dbattenuationatmax _attenuationshapeextents _coneoffset _falloffdistance) (break `SoundAttenuationSettings` _outattenuationsettings))
  (`AudioComponent.AdjustAttenuation` _audiounderwater_2 (make `SoundAttenuationSettings` _battenuate _bspatialize _battenuatewithlpf _benablelistenerfocus _benablefocusinterpolation _benableocclusion _busecomplexcollisionforocclusion _benablereverbsend _bapplynormalizationtostereosounds _benablelogfrequencyscaling _omniradius _stereospread _spatializationalgorithm null _lpfradiusmin _lpfradiusmax _absorptionmethod _customlowpassairabsorptioncurve _customhighpassairabsorptioncurve _lpffrequencyatmin _lpffrequencyatmax _hpffrequencyatmin _hpffrequencyatmax _focusazimuth _nonfocusazimuth _focusdistancescale _nonfocusdistancescale _focuspriorityscale _nonfocuspriorityscale _focusvolumeattenuation _nonfocusvolumeattenuation _focusattackinterpspeed _focusreleaseinterpspeed _occlusiontracechannel _occlusionlowpassfilterfrequency _occlusionvolumeattenuation _occlusioninterpolationtime null _reverbsendmethod null _reverbwetlevelmin _reverbwetlevelmax _reverbdistancemin _reverbdistancemax _customreverbsendcurve _manualreverbsendlevel _distancealgorithm _customattenuationcurve _attenuationshape _dbattenuationatmax (* (`self.VolumeBoxExtend`) (`SceneComponent.K2_GetComponentScale` (`self.Root`))) _coneoffset _falloffdistance))
  (`SceneComponent.SetRelativeScale3D` _audiounderwater (1.0 1.0 1.0))
  (`SceneComponent.K2_SetRelativeLocation` _audiounderwater (+ (`self.VolumeBoxLocation`) (`KismetMathLibrary.MakeVector` 0.0 0.0 (+ (* -1 (.z (`self.VolumeBoxExtend`))) (* _falloffdistance -0.5)))) false false))

(fn `UpdateCubemapParameters`
  (`self.BoxReflection` (`self.ReflectionOver`) (`self.OverWaterMaterialInstance`) (`self.ReflectionBoxOverExtend`) (`self.ReflectionBoxOverLocation`) true)
  (`self.BoxReflection` (`self.ReflectionUnder`) (`self.UnderWaterMaterialInstance`) (`self.ReflectionBoxUnderExtend`) (`self.ReflectionBoxUnderLocation`)))

(fn `UpdateHoles`
  (locals (CleanTransform :type "Transform Structure" :default "100000.000000,100000.000000,0.000000|0.000000,0.000000,0.000000|1.000000,1.000000,1.000000") (CleanOffset :type "Vector2D Structure" :default (0.0 0.0)) (SleanScale :type "Vector2D Structure" :default (0.001 0.001)))
  (for _index (range 1 6)
    (`/Game/AquaticSurface/Blueprints/BP_AquaticLibrary.CutHole` _index (`local.CleanTransform`) (`local.CleanOffset`) (`local.SleanScale`)))
  (`KismetArrayLibrary.Array_RemoveItem` (`self.Holes`))
  (for _array_element (`self.Holes`)
    (`/Engine/EditorBlueprintResources/StandardMacros.IsValid` _array_element
      (:`Is Valid`
        (`/Game/AquaticSurface/Blueprints/BP_AquaticHole.UpdateCutHole` _array_element)))))

(fn `UpdateInteractionComponent`
  (params (Location :type "Vector2D Structure") (InteractionRadius :type "Float (double-precision)"))
  (bind (_x _y) (`KismetMathLibrary.BreakVector2D` Location))
  (bind (_returnvalue_x _returnvalue_y _returnvalue_z) (`KismetMathLibrary.BreakVector` (`self.K2_GetActorLocation`)))
  (bind _interactionradius (`local.InteractionRadius`))
  (bind (_origin _boxextent) (`KismetSystemLibrary.GetComponentBounds` (`self.PlaneOverWater`)))
  (bind _returnvalue (`KismetMathLibrary.MakeVector` (`KismetMathLibrary.FMin` _interactionradius (.x _boxextent)) (`KismetMathLibrary.FMin` _interactionradius (.y _boxextent)) 10.0))
  (bind _returnvalue_2 (- _boxextent _returnvalue))
  (bind (_returnvalue_x_2 _returnvalue_y_2) (`KismetMathLibrary.BreakVector` (- _origin _returnvalue_2)))
  (bind (_returnvalue_x_3 _returnvalue_y_3) (`KismetMathLibrary.BreakVector` (+ _returnvalue_2 _origin)))
  ;[1 1 1] Calculate position on surface.
  (`SceneComponent.SetWorldScale3D` (`self.InteractionView`) _returnvalue)
  (`SceneComponent.K2_SetWorldLocation` (`self.InteractionView`) (`KismetMathLibrary.MakeVector` (`KismetMathLibrary.FClamp` _x _returnvalue_x_2 _returnvalue_x_3) (`KismetMathLibrary.FClamp` _y _returnvalue_y_2 _returnvalue_y_3) _returnvalue_z) false false))

(fn `UpdatePostProcessShape`
  (locals (PositionShift :type "Float (double-precision)" :default 15.0))
  (bind _postprocessmesh (`self.PostProcessMesh`))
  (bind _postprocessshape (`self.PostProcessShape`))
  (bind _positionshift (`local.PositionShift`))
  ;[1 1 1] Box volume ostprocess settings
  (`MaterialInstanceDynamic.SetScalarParameterValue` (`self.ScreenMaterialIntance`) "WaterHeight" (`self.GetHeight`))
  (`MaterialInstanceDynamic.SetScalarParameterValue` (`self.VolumeMaterialInstance`) "WaterHeight" (`self.GetHeight`))
  (`SceneComponent.SetRelativeScale3D` _postprocessmesh (* (- (`self.VolumeBoxExtend`) (`KismetMathLibrary.MakeVector` 0.0 0.0 (* _positionshift 0.5))) 0.02))
  (`SceneComponent.K2_SetRelativeLocation` _postprocessmesh (`KismetMathLibrary.MakeVector` 0.0 0.0 (* _positionshift -0.5)) false false)
  ;[1 1 1] Collision shape settings
  (`BoxComponent.SetBoxExtent` _postprocessshape (`self.VolumeBoxExtend`) true)
  (`SceneComponent.SetRelativeScale3D` _postprocessshape (1.0 1.0 1.0))
  (`SceneComponent.K2_SetRelativeLocation` _postprocessshape (+ (`self.VolumeBoxLocation`) (`KismetMathLibrary.MakeVector` 0.0 0.0 (+ (* -1 (.z (`self.VolumeBoxExtend`))) (`local.PositionShift`)))) false false))

(fn `UpdateReflectionShape`
  (bind _capturecube (`self.CaptureCube`))
  (bind _hiddeninreflection (`self.HiddenInReflection`))
  (bind _returnvalue (/ (`self.ReflectionLocation`) (`SceneComponent.RelativeScale3D` (`self.Root`))))
  (if (`KismetSystemLibrary.IsValid` (`self.ReflectionExternal`))
    ;[1 1 1] External reflection actor
    (set `self.ReflectionLocation` (- (`SceneComponent.K2_GetComponentLocation` (`SceneCaptureCube.CaptureComponentCube` (`self.ReflectionExternal`))) (`self.K2_GetActorLocation`)))
    (else
      (`/Engine/EditorBlueprintResources/StandardMacros.IsValid` (`self.StaticReflectionCubemap`)
        (:`Is Valid`
          (`/Engine/EditorBlueprintResources/StandardMacros.IsValid` _capturecube
            (:`Is Valid`
              (`ActorComponent.K2_DestroyComponent` _capturecube))))
        (:`Is Not Valid`
          ;[1 1 1] Build in reflection actor
          (`SceneComponent.K2_SetRelativeTransform` (`self.CaptureCube`) (`KismetMathLibrary.MakeTransform` _returnvalue) false false)
          (`SceneComponent.SetWorldScale3D` (`self.CaptureCube`) (1.0 1.0 1.0))
          (`KismetArrayLibrary.Array_AddUnique` _hiddeninreflection self)
          (set `SceneCaptureComponent.HiddenActors` _hiddeninreflection (`self.CaptureCube`))
          (`SceneCaptureComponentCube.CaptureScene` (`self.CaptureCube`))))))
  ;[1 1 1] Create reflections
  (`SceneComponent.K2_SetRelativeLocation` (`self.ReflectionBillboad`) _returnvalue false false))

(fn `UpdateVolume`
  (bind _returnvalue (`MaterialInstanceDynamic.K2_GetScalarParameterValue` (`self.VolumeMaterialInstance`) "FogBase"))
  (set `self.VolumeFogBase` _returnvalue)
  (bind _returnvalue_2 (`MaterialInstanceDynamic.K2_GetScalarParameterValue` (`self.VolumeMaterialInstance`) "FogDensity"))
  (set `self.VolumeFogDensity` _returnvalue_2)
  (`KismetMaterialLibrary.SetScalarParameterValue` "/Game/AquaticSurface/Materials/PC_AquaticSurface.PC_AquaticSurface" "FogBase" (`self.VolumeFogBase`))
  (`KismetMaterialLibrary.SetScalarParameterValue` "/Game/AquaticSurface/Materials/PC_AquaticSurface.PC_AquaticSurface" "FogDenisty" (`self.VolumeFogDensity`))
  (`KismetMaterialLibrary.SetScalarParameterValue` "/Game/AquaticSurface/Materials/PC_AquaticSurface.PC_AquaticSurface" "CurrentWaterHeight" (.z (`SceneComponent.K2_GetComponentLocation` (`self.Root`)))))

(fn `UserConstructionScript`
  (`self.Reconstruct`)
  (`self.UpdateHoles`))