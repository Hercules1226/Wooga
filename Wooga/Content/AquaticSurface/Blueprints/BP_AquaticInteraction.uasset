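; BP_AquaticInteraction supplies the transform, fade and splash flag for an object's interaction with an aquatic surface.
; GetTransform is an overridable getter that fades by vertical distance to the surface root, at full strength within half of MaxSurfaceDistance and zero at that distance.
; SetInHole maintains a counter of holes, and any nonzero count, like being disabled, zeroes the fade and turns off splashing.
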(fn `GetTransform`
  (params (Surface :type "/Game/AquaticSurface/Blueprints/BP_AquaticSurface Object Reference"))
  (returns (Location :type "Vector Structure") (Rotation :type "Rotator Structure") (Fade :type "Float (double-precision)") (Splash :type Boolean))
  (bind (_returnvalue_location _returnvalue_rotation) (`KismetMathLibrary.BreakTransform` (`self.K2_GetComponentToWorld`)))
  (bind _maxsurfacedistance (`self.MaxSurfaceDistance`))
  (bind (_returnvalue_x _returnvalue_y _returnvalue_z) (`KismetMathLibrary.BreakVector` (`self.K2_GetComponentLocation` (`/Game/AquaticSurface/Blueprints/BP_AquaticSurface.Root` Surface))))
  ;[1 1 1] You can implement your own location and rotation getter here.
  (if (and (`self.Enabled`) (== (`self.InHole`) 0))
    (return _returnvalue_location _returnvalue_rotation (`KismetMathLibrary.MapRangeClamped` (`KismetMathLibrary.Abs` (- _returnvalue_z (.z _returnvalue_location))) _maxsurfacedistance (* _maxsurfacedistance 0.5) 0.0 1.0) true)
    (else
      (return _returnvalue_location _returnvalue_rotation 0.0 false))))

(fn `SetInHole`
  (params (Increase :type Boolean))
  (if Increase
    (`/Engine/EditorBlueprintResources/StandardMacros.IncrementInt` (`self.InHole`))
    (else
      (`/Engine/EditorBlueprintResources/StandardMacros.DecrementInt` (`self.InHole`)))))