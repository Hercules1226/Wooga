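; Buoyancy component that floats its owner's physics-simulating primitive in an aquatic surface volume.
; SetAquaticVolume toggles tick and swaps the mesh between water-scaled and cached damping.
; Each tick measures depth below the volume's flat Z, derives a cylinder, sphere or cone cap volume, and applies scaled upward force at CenterOfMass.
; Force is skipped on world origin shifts; hole counting exists, but its reactivation is empty.
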(event `self.ReceiveBeginPlay`
  (`self.SetComponentTickEnabled` false)
  (`self.ValidateMesh`)
  (`self.SetAquaticVolume` (`self.InWater`)))

(event `self.ReceiveTick`
  (params (DeltaSeconds :type "Float (single-precision)"))
  ;[1 1 1] Ticked only when object is in the water (there is no other way in the blueprints
  (`self.UpdateInFluid` DeltaSeconds))

(fn `GetSurfceDistance`
  (params (Location :type "Vector Structure"))
  (returns (Distance :type "Float (double-precision)"))
  (bind _inwater (`self.InWater`))
  (bind (_returnvalue_x _returnvalue_y _returnvalue_z) (`KismetMathLibrary.BreakVector` (`Actor.K2_GetActorLocation` _inwater)))
  (`/Engine/EditorBlueprintResources/StandardMacros.IsValid` _inwater
    (:`Is Valid`
      (return (+ (- _returnvalue_z (.z Location)) (`self.ShapeRadius`))))
    (:`Is Not Valid`
      (return -100000.0))))

(fn `IsEnabled`
  (returns (IsEnabled :type Boolean))
  (return (and (`self.Enabled`) (<= (`self.HoleCount`) 0))))

(fn `SetAquaticVolume`
  (params (AquaticSurface :type "/Game/AquaticSurface/Blueprints/BP_AquaticSurface Object Reference"))
  (bind _output_get (set `self.InWater` AquaticSurface))
  (`self.SetTickMode` (`KismetSystemLibrary.IsValid` _output_get))
  (`/Engine/EditorBlueprintResources/StandardMacros.IsValid` (`self.InWater`)
    (:`Is Valid`
      (`/Engine/EditorBlueprintResources/StandardMacros.IsValid` (`Actor.GetComponentByClass` (`self.GetOwner`) "/Script/Engine.CharacterMovementComponent")))))

(fn `SetInHole`
  (params (Increase :type Boolean))
  (bind _holecount (`self.HoleCount`))
  (if Increase
    (`/Engine/EditorBlueprintResources/StandardMacros.IncrementInt` _holecount)
    (else
      (bind _result (`/Engine/EditorBlueprintResources/StandardMacros.DecrementInt` _holecount)
        (:`  `
          (if (== _result 0)
            (`self.TryReactivate`)))))))

(fn `SetTickMode`
  (params (InWater :type Boolean))
  (bind _cachedmesh (`self.CachedMesh`))
  (bind _cachedmesh_2 (`self.CachedMesh`))
  (`self.SetComponentTickEnabled` InWater)
  (if (`KismetSystemLibrary.IsValid` (`self.CachedMesh`))
    (if InWater
      (`PrimitiveComponent.SetLinearDamping` _cachedmesh (* (`self.LinearDampingScale`) (`/Game/AquaticSurface/Blueprints/BP_AquaticSurface.BuoyancyLinearDamping` (`self.InWater`))))
      (`PrimitiveComponent.SetAngularDamping` _cachedmesh (* (`self.AngularDampingScale`) (`/Game/AquaticSurface/Blueprints/BP_AquaticSurface.BuoyancyAngularDamping` (`self.InWater`))))
      (else
        (`PrimitiveComponent.SetLinearDamping` _cachedmesh_2 (`self.LinearDampingCached`))
        (`PrimitiveComponent.SetAngularDamping` _cachedmesh_2 (`self.AngularDampingCached`))))))

(fn `TryReactivate`)

(fn `UpdateInFluid`
  (params (DeltaTime :type "Float (double-precision)"))
  (locals (BuoyancyForce :type "Float (double-precision)"))
  (bind (_returnvalue_x _returnvalue_y _returnvalue_z) (break `IntVector` (`GameplayStatics.GetWorldOriginLocation`)))
  (bind (_prevworldoriginlocation_x _prevworldoriginlocation_y _prevworldoriginlocation_z) (break `IntVector` (`self.PrevWorldOriginLocation`)))
  (bind _distance (`self.GetSurfceDistance` (`SceneComponent.K2_GetComponentLocation` (`self.CachedMesh`))))
  (if (and (and (== _returnvalue_x _prevworldoriginlocation_x) (== _returnvalue_y _prevworldoriginlocation_y)) (== _returnvalue_z _prevworldoriginlocation_z))
    (`/Engine/EditorBlueprintResources/StandardMacros.IsValid` (`self.CachedMesh`)
      (:`Is Valid`
        (if (> _distance 0.0)
          ;[1 1 1] Calculate frce
          (`|ExecutionSequence`
            (:`then_0`
              (switch `/Game/AquaticSurface/Blueprints/BuoyancyShape` (`self.Shape`)
                (:`NewEnumerator0`
                  (set `local.BuoyancyForce` (`self.CylinderCapVolume` _distance (`self.ShapeRadius`))))
                (:`NewEnumerator1`
                  (set `local.BuoyancyForce` (`self.SphereCapVolume` _distance (`self.ShapeRadius`))))
                (:`NewEnumerator2`
                  (set `local.BuoyancyForce` (`self.ConeCapVolume` _distance (`self.ShapeRadius`))))))
            (:`then_1`
              ;[1 1 1] Apply force
              (`PrimitiveComponent.AddForceAtLocation` (`self.CachedMesh`) (`KismetMathLibrary.MakeVector` 0.0 0.0 (* (`local.BuoyancyForce`) (`self.FinalForce`))) (`KismetMathLibrary.TransformLocation` (`SceneComponent.K2_GetComponentToWorld` (`self.CachedMesh`)) (`self.CenterOfMass`)) "None"))))))
    (else
      (set `self.PrevWorldOriginLocation` (`GameplayStatics.GetWorldOriginLocation`)))))

(fn `ValidateMesh`
  (bind _cachedmesh (`self.CachedMesh`))
  (bind _returnvalue (`Actor.GetComponentByClass` (`self.GetOwner`) "/Script/Engine.PrimitiveComponent"))
  ;[1 1 1] Looking for physics component
  (if (`SceneComponent.IsSimulatingPhysics` _returnvalue "None")
    (bind _output_get (set `self.CachedMesh` _returnvalue))
    (set `self.FinalForce` (* (`KismetMathLibrary.Dot_VectorVector` (`SceneComponent.K2_GetComponentScale` _output_get) (0.333 0.333 0.333)) (`self.ForceScale`)))
    ;[1 1 1] Cache damping parameters
    (`/Engine/EditorBlueprintResources/StandardMacros.IsValid` _cachedmesh
      (:`Is Valid`
        (set `self.AngularDampingCached` (`PrimitiveComponent.GetAngularDamping` _cachedmesh))
        (set `self.LinearDampingCached` (`PrimitiveComponent.GetLinearDamping` _cachedmesh))))))